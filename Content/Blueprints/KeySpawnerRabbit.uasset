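; KeySpawnerRabbit is a slappable actor, by its name a rabbit variant, that can drop a key when slapped.
; It overrides Slap, calling the parent version first and then checking KeyCount on BGGameInstance.
; With no keys counted, it spawns a KeyActor at KeySpawnLocation's transform and appends a drop notice to the parent's returned text; otherwise it returns that text unchanged.
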(fn `Slap`
  (returns (CombatLog :type String))
  (bind _combatlog (`parent.Slap`))
  (bind _asbggame_instance (cast `/Game/Blueprints/BGGameInstance` (`GameplayStatics.GetGameInstance`)))
  (if (>= (`/Game/Blueprints/BGGameInstance.KeyCount` _asbggame_instance) 1)
    (return _combatlog)
    (else
      (`|SpawnActorFromClass` "/Game/Blueprints/KeyActor.KeyActor_C" (`self.GetTransform` (`self.KeySpawnLocation`)) "Undefined" "OverrideRootScale" null null)
      (return (`KismetStringLibrary.Concat_StrStr` _combatlog " It dropped a key!")))))

(fn `UserConstructionScript`
  (`parent.UserConstructionScript`))