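; Conversation actor for Boggledoop, an NPC who joins the player's team after being slapped repeatedly.
; Slap steps through dialogue lines with a slap counter, playing a sound and returning each line as a string.
; The final step spawns a BoogledoopCharacter at the actor's transform and sets TeamSize to 3 in BGGameInstance.
; Once TeamSize is 3, Slap returns only an idle line.
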(fn `Slap`
  (returns (ConsoleMessage :type String))
  (bind _asbggame_instance (cast `/Game/Blueprints/BGGameInstance` (`GameplayStatics.GetGameInstance`)))
  (if (== (`/Game/Blueprints/BGGameInstance.TeamSize` _asbggame_instance) 3)
    (return "Gagglesnoop: I come drink often here.")
    (elif (<= (`self.SlapCount`) 7)
      (`AudioComponent.Play` (`self.DialogueSounds`) 0.0)
      (bind _result (`/Engine/EditorBlueprintResources/StandardMacros.IncrementInt` (`self.SlapCount`))
        (:`  `
          (switch `int` _result
            (:`Default`
              (return "Gagglesnoop: I come drink often here."))
            (:`0`
              (return "Boogledoop: YAAAAAAAAAAAY"))
            (:`1`
              (return "Gobbleboop: I am Poddledug!"))
            (:`2`
              (return "Mooglegoop: Your ze hands are so softy!"))
            (:`3`
              (return "Bobbledoof: I must now your secret for ze hands!"))
            (:`4`
              (return "Parflefloof: I am follow you yaaaaaaaay!"))
            (:`5`
              (return "GAFFLESNOOF: YAAAAAAAAAAAAAAAAAAAY!"))
            (:`6`
              (`|SpawnActorFromClass` (`self.BoogledoopCharacter`) (`self.GetTransform`) "Undefined" "OverrideRootScale" null null)
              (bind _asbggame_instance_2 (cast `/Game/Blueprints/BGGameInstance` (`GameplayStatics.GetGameInstance`)))
              (set `/Game/Blueprints/BGGameInstance.TeamSize` 3 _asbggame_instance_2)
              (return "Boggledoop joined the bande!"))))))))

(fn `UserConstructionScript`
  (`parent.UserConstructionScript`))