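; BGGameInstance is a Game Instance Blueprint that sets up a level's UI and the player's team.
; SetupLevel adds GameUI to the viewport and caches player 0's 2DSideScrollerCharacter as MrHero.
; TeamSize then determines which companions spawn at the player's transform: WizardMcWizfaceCharacter joins first, and BoogledoopCharacter follows for larger teams.
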(fn `SetupLevel`
  (bind _teamsize (`self.TeamSize`))
  (bind _returnvalue (`Actor.GetTransform` (`GameplayStatics.GetPlayerCharacter` 0)))
  ;[1 1 1] Setup UI
  (`UserWidget.AddToViewport` (`self.GameUI`) 0)
  ;[1 1 1] Setup team
  (bind _as2dside_scroller_character (cast `/Game/2DSideScrollerBP/Blueprints/2DSideScrollerCharacter` (`GameplayStatics.GetPlayerCharacter` 0)))
  (set `self.MrHero` _as2dside_scroller_character)
  (if (>= _teamsize 2)
    (`|SpawnActorFromClass` "/Game/Blueprints/WizardMcWizfaceCharacter.WizardMcWizfaceCharacter_C" _returnvalue "Undefined" "OverrideRootScale" null null)
    (if (>= _teamsize 3)
      (`|SpawnActorFromClass` "/Game/Blueprints/BoogledoopCharacter.BoogledoopCharacter_C" _returnvalue "Undefined" "OverrideRootScale" null null))))