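; RabbitPawn is a 2D Paper flipbook rabbit that wanders sideways and can be slapped dead.
; Tick alternates a random-length wait with a fixed-length run along X, swapping flipbooks and updating the MoveRight direction after each run.
; Movement counts ticks and steps a fixed distance without sweep, so speed depends on frame rate.
; Slap stops it, shows the dead flipbook and returns a randomized joke combat log, or a quip if already dead.
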(event `self.ReceiveTick`
  (params (DeltaSeconds :type "Float (single-precision)"))
  (bind _movingticksleft (`self.MovingTicksLeft`))
  (if (`self.IsDead`)
    _
    (elif (`self.IsMoving`)
      ;[1 1 1] Move
      (`self.K2_SetActorLocation` (`KismetMathLibrary.MakeVector` (+ (.x (`self.K2_GetActorLocation`)) (`KismetMathLibrary.Conv_IntToDouble` (* (`self.MoveRight`) 3))) (.y (`self.K2_GetActorLocation`)) (.z (`self.K2_GetActorLocation`))))
      (bind _result (`/Engine/EditorBlueprintResources/StandardMacros.DecrementInt` _movingticksleft)
        (:`  `
          (set `self.MovingTicksLeft` _result)
          (if (<= _movingticksleft 0)
            (`PaperFlipbookComponent.SetFlipbook` (`self.PaperFlipbook`) "/Game/Flipbooks/Rabbit_Flipbook.Rabbit_Flipbook")
            (set `self.IsMoving` false)
            (set `self.MovingTicksLeft` (`self.MovingTicks`))
            (bind _result_2 (`/Engine/EditorBlueprintResources/StandardMacros.NegateInt` (`self.MoveRight`))
              (:`  `
                (set `self.MoveRight` _result_2))))))
      (else
        ;[1 1 1] Wait
        (bind _result_3 (`/Engine/EditorBlueprintResources/StandardMacros.DecrementInt` (`self.WaitingTicksLeft`))
          (:`  `
            (bind _output_get (set `self.WaitingTicksLeft` _result_3))
            (if (<= _output_get 0)
              (`PaperFlipbookComponent.SetFlipbook` (`self.PaperFlipbook`) "/Game/Flipbooks/RabbitRun.RabbitRun")
              (set `self.IsMoving` true)
              (set `self.WaitingTicksLeft` (`KismetMathLibrary.RandomIntegerInRange` (`self.WaitingTicksMin`) (`self.WaitingTicksMax`))))))))))

(fn `Slap`
  (returns (CombatLog :type String))
  (bind _goobledoopnames (`self.GoobledoopNames`))
  (if (`self.IsDead`)
    (return "Poor rabbit looks very deaded.")
    (else
      (set `self.IsDead` true)
      (`PaperFlipbookComponent.SetFlipbook` (`self.PaperFlipbook`) "/Game/Flipbooks/RabbitDead_Flipbook.RabbitDead_Flipbook")
      (return (`KismetStringLibrary.Concat_StrStr` "MrHero slaps for " (`KismetStringLibrary.Conv_IntToString` (`KismetMathLibrary.RandomIntegerInRange` 20 60)) " physical damage. Wizard McWizface magics for " (`KismetStringLibrary.Conv_IntToString` (`KismetMathLibrary.RandomIntegerInRange` 30 40)) "  arcane damage. " (`|GetArrayItem` _goobledoopnames (`KismetMathLibrary.RandomIntegerInRange` 0 (`KismetArrayLibrary.Array_Length` _goobledoopnames))) " whatevers for " (`KismetStringLibrary.Conv_IntToString` (`KismetMathLibrary.RandomIntegerInRange` 1 99)) " tructruc damage. Rabbit falls!")))))

(fn `UserConstructionScript`)