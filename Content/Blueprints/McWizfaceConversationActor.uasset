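; McWizfaceConversationActor is a slappable door in a comedic game that plays the recruitment scene for Wizard McWizface.
; Each Slap call increments a counter and returns the next line of dialogue through a switch, falling back to a no-effect message once the script runs out.
; Along the way it reveals a stand-in animation actor, then hides it and spawns McWizfaceCharacter at its transform as he joins the party.
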(fn `Slap`
  (returns (ConsoleMessage :type String))
  (bind _mcwizfaceanimationactor (`self.McWizfaceAnimationActor`))
  (bind _result (`/Engine/EditorBlueprintResources/StandardMacros.IncrementInt` (`self.SlapCount`))
    (:`  `
      (switch `int` _result
        (:`Default`
          (return "MrHero slaps ze door gentle. But nothing happen."))
        (:`0`
          (return "MrHero slaps ze wierd door handle. It wiggles nicely. Someone is inside making noises!"))
        (:`1`
          (return "Wizardly voice: WHAT IS IT I AM A BUSY PERSON"))
        (:`2`
          (return "Wizardly voice: I SWEAR YOU PUNK IF YOU SLAP ZIS HANDLE AGAIN I'LL DO THINGS"))
        (:`3`
          (`self.SetActorHiddenInGame` (`self.McWizfaceAnimationActor`) false)
          (return "Wizard McWizface: HERE I COMME"))
        (:`4`
          (return "Wizard McWizface: Oh it's you MrHero!"))
        (:`5`
          (return "Wizard McWizface: You louke very heroique today!"))
        (:`6`
          (return "Wizard McWizface: I should come wif you!"))
        (:`7`
          (`self.SetActorHiddenInGame` _mcwizfaceanimationactor true)
          (`|SpawnActorFromClass` (`self.McWizfaceCharacter`) (`self.GetTransform` _mcwizfaceanimationactor) "Undefined" "OverrideRootScale" null null)
          (return "WizardMcWizface joined the bande!"))))))

(fn `UserConstructionScript`
  (`parent.UserConstructionScript`))