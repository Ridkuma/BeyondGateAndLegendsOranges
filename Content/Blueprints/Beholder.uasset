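; Beholder quest-giver NPC whose dialogue advances each time it is slapped, sending the player to find lost keys in exchange for Michou's game.
; Slap plays a sound and returns the next line, using a shared SlapCount switch to step through the intro until HaveQuest is set.
; It then repeats a reminder while the game instance's KeyCount is zero; otherwise it continues into the completion dialogue and opens the Ending level.
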(fn `Slap`
  (returns (ConsoleMessage :type String))
  (locals (KeyCountLocal :type Integer :default 0))
  (bind _asbggame_instance (cast `/Game/Blueprints/BGGameInstance` (`GameplayStatics.GetGameInstance`)))
  (set `self.KeyCount` (`/Game/Blueprints/BGGameInstance.KeyCount` _asbggame_instance))
  (`AudioComponent.Play` (`self.DialogueSounds`) 0.0)
  (if (`self.HaveQuest`)
    (if (== (`self.KeyCount`) 0)
      _
      (else
        ;[1 1 1] Quest complete
        (bind _result (`/Engine/EditorBlueprintResources/StandardMacros.IncrementInt` (`self.SlapCount`))
          (:`  `
            (switch `int` _result
              (:`11`
                (return "MrHero slaps the key on the Beholder's face."))
              (:`12`
                (return "Beholder: My, my, my, color me impressed!"))
              (:`13`
                (return "Beholder: Thank you very much, brave heroes, you certainly did not waste an hour playing this dumb game."))
              (:`14`
                (return "Beholder: I will just head in a make some hot cocoa, but I am just going to teleport you guys back to Michou, he must be distraught."))
              (:`15`
                (return "Beholder:Feel free to drop by anytime though! Farewell!"))
              (:`16`
                _)
              (:`17`
                (`GameplayStatics.OpenLevel` "Ending")))
            (return "You feel magicks everywere in you bodies. It feelz fuzzy. Or fussy. Or bothe. And ze Beholder slaps you one last time.")))))
    (else
      ;[1 1 1] Give and wait for quest
      (bind _result_2 (`/Engine/EditorBlueprintResources/StandardMacros.IncrementInt` (`self.SlapCount`))
        (:`  `
          (switch `int` _result_2
            (:`Default`
              (return "Beholder: Oh, hi gentlemen. I see you are already familiar with the customs of my people."))
            (:`0`
              (return "Beholder: Oh, hi gentlemen. I see you are already familiar with the customs of my people."))
            (:`1`
              (return "The Beholder gently carresses your faces with a kind eye."))
            (:`2`
              (return "Beholder: I take it you fine people are here on the behalf of Michou?"))
            (:`3`
              (return "Beholder: Yes, I do have his game's master copy."))
            (:`4`
              (return "Beholder: I actually tried it. That's all I wanted. Reality check and all, I am sure you know how it is."))
            (:`5`
              (return "Beholder: And yes, I am willing to give it back to you guys."))
            (:`6`
              (return "Beholder: HOWEVER."))
            (:`7`
              (return "Beholder: You don't seem to have better to do than running around."))
            (:`8`
              (return "Beholder: And I seem to have misplaced my keys in the forest. Surely one of those damn rabbits have them."))
            (:`9`
              (return "Beholder: If you would be so kind as to bring them to me, I will part with Michou's game."))
            (:`10`
              (set `self.HaveQuest` true)))))))
  (return "Beholder: Return to me when you have them, will you? I am positively certain they are around. That will be today's quest."))

(fn `UserConstructionScript`
  (`parent.UserConstructionScript`))