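; Player hero character that moves along the world X axis and plays sounds for footsteps, jumping and slapping.
; MoveRight input tracks facing through BisMovingRight, adds movement and starts the footsteps cue whenever it is not already playing, even at zero input.
; Tick calls DefaultTick, then stops footsteps when the hero is not moving or is falling.
; WhenJumping plays the jump cue, and the SlapStuff override runs the parent logic before playing slap sounds.
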(event `InputAxis|MoveRight`
  (params (AxisValue :type "Float (single-precision)"))
  (bind _footstepscue (`self.FootstepsCue`))
  ;[1 1 1] Handle movement
  (if (> AxisValue 0.0)
    (set `self.bisMovingRight` true)
    (elif (< AxisValue 0.0)
      (set `self.bisMovingRight` false)))
  (`self.AddMovementInput` (1.0 0.0 0.0) AxisValue)
  (if (not (`AudioComponent.IsPlaying` _footstepscue))
    (`AudioComponent.Play` _footstepscue 0.0)))

(event `self.ReceiveTick`
  (params (DeltaSeconds :type "Float (single-precision)"))
  (bind _footstepscue (`self.FootstepsCue`))
  (bind _returnvalue (`AudioComponent.IsPlaying` _footstepscue))
  (`self.DefaultTick`)
  (`/Engine/EditorBlueprintResources/StandardMacros.IsValid` _footstepscue
    (:`Is Valid`
      (if (or (and _returnvalue (not (`self.IsMoving`))) (and _returnvalue (`self.IsFalling`)))
        (`AudioComponent.Stop` (`self.FootstepsCue`))))))

(event `self.WhenJumping`
  (`AudioComponent.Play` (`self.JumpCue`) 0.0))

(fn `SlapStuff`
  (returns (NewParam :type String))
  (bind _newparam (`parent.SlapStuff`))
  (`AudioComponent.Play` (`self.SlapSounds`) 0.0)
  (return _newparam))

(fn `UserConstructionScript`
  (`parent.UserConstructionScript`))