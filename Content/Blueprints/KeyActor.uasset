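; KeyActor is a collectible key that the player picks up by slapping it.
; Its Slap override calls the parent, increments KeyCount on the BGGameInstance, then destroys the actor and returns a flavor line about MrHero and a jealous Goobledoop.
; The event graph holds only disabled default events, so all behavior lives in Slap.
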(fn `Slap`
  (returns (ConsoleMessage :type String))
  (`parent.Slap`)
  (bind _asbggame_instance (cast `/Game/Blueprints/BGGameInstance` (`GameplayStatics.GetGameInstance`)))
  (`/Engine/EditorBlueprintResources/StandardMacros.IncrementInt` (`/Game/Blueprints/BGGameInstance.KeyCount` _asbggame_instance)
    (:`  `
      (`self.K2_DestroyActor`)
      (return "MrHero slaps a key. Goobledoop looks jealous."))))

(fn `UserConstructionScript`
  (`parent.UserConstructionScript`))